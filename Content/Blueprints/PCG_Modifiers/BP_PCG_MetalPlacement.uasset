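; BP_PCG_MetalPlacement is a PCG modifier actor for placing one of three metal mesh variants.
; Its construction script clears the actor's tags, then uses Variant to add the matching Metal_Type tag and set the static mesh.
; The Box component is then resized to that mesh component's bounds extent.
; It has no active runtime logic.
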(event EventBeginPlay)

(event Collision|EventActorBeginOverlap
  (params (OtherActor :type Actor%20Object%20Reference)))

(event EventTick
  (params (DeltaSeconds :type Float%20%28single-precision%29)))

(fn ConstructionScript
  (Utilities|Array|Clear (Variables|Actor|GetTags))
  (switch int (Variables|EditorSelection|GetVariant)
    (:1
      (Utilities|Array|AddUnique (Variables|Actor|GetTags) "Metal_TypeA")
      (Components|StaticMesh|SetStaticMesh (Variables|Default|GetStaticMesh) "/Game/Assets/Meshes/ResourceNodes/SM_Metal_A.SM_Metal_A"))
    (:2
      (Utilities|Array|AddUnique (Variables|Actor|GetTags) "Metal_TypeB")
      (Components|StaticMesh|SetStaticMesh (Variables|Default|GetStaticMesh) "/Game/Assets/Meshes/ResourceNodes/SM_Metal_B.SM_Metal_B"))
    (:3
      (Utilities|Array|AddUnique (Variables|Actor|GetTags) "Metal_TypeC")
      (Components|StaticMesh|SetStaticMesh (Variables|Default|GetStaticMesh) "/Game/Assets/Meshes/ResourceNodes/SM_Metal_C.SM_Metal_C")))
  (Components|Box|SetBoxExtent (Variables|Default|GetBox) (.BoxExtent (Collision|GetComponentBounds (Variables|Default|GetStaticMesh))) true))