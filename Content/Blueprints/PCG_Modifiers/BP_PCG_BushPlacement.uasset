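; Placeable berry bush actor in the PCG modifiers set, offering five bush variants selected by the Variant value.
; The construction script clears the actor tags, then adds the matching Bush_Type tag and assigns that variant's static mesh.
; It then resizes the Box component to the mesh's bounds extent.
; All logic runs at construction, as the event graph holds only disabled stub events.
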(event EventBeginPlay)

(event Collision|EventActorBeginOverlap
  (params (OtherActor :type Actor%20Object%20Reference)))

(event EventTick
  (params (DeltaSeconds :type Float%20%28single-precision%29)))

(fn ConstructionScript
  (Utilities|Array|Clear (Variables|Actor|GetTags))
  (switch int (Variables|EditorSelection|GetVariant)
    (:1
      (Utilities|Array|AddUnique (Variables|Actor|GetTags) "Bush_TypeA")
      (Components|StaticMesh|SetStaticMesh (Variables|Default|GetStaticMesh) "/Game/Assets/Meshes/Bushes/berry-bush-a-full.berry-bush-a-full"))
    (:2
      (Utilities|Array|AddUnique (Variables|Actor|GetTags) "Bush_TypeB")
      (Components|StaticMesh|SetStaticMesh (Variables|Default|GetStaticMesh) "/Game/Assets/Meshes/Bushes/berry-bush-b-full.berry-bush-b-full"))
    (:3
      (Utilities|Array|AddUnique (Variables|Actor|GetTags) "Bush_TypeC")
      (Components|StaticMesh|SetStaticMesh (Variables|Default|GetStaticMesh) "/Game/Assets/Meshes/Bushes/berry-bush-c-full.berry-bush-c-full"))
    (:4
      (Utilities|Array|AddUnique (Variables|Actor|GetTags) "Bush_TypeD")
      (Components|StaticMesh|SetStaticMesh (Variables|Default|GetStaticMesh) "/Game/Assets/Meshes/Bushes/berry-bush-d-full.berry-bush-d-full"))
    (:5
      (Utilities|Array|AddUnique (Variables|Actor|GetTags) "Bush_TypeE")
      (Components|StaticMesh|SetStaticMesh (Variables|Default|GetStaticMesh) "/Game/Assets/Meshes/Bushes/berry-bush-e-full.berry-bush-e-full")))
  (Components|Box|SetBoxExtent (Variables|Default|GetBox) (.BoxExtent (Collision|GetComponentBounds (Variables|Default|GetStaticMesh))) true))