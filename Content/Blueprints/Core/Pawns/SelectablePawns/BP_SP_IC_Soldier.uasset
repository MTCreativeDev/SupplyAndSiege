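; Selectable soldier pawn Blueprint that shows a selection ring and team-colored materials.
; On BeginPlay it runs the parent logic and binds the UnitInformationComponent's selection-ring event to toggle UnitSelectionRing visibility.
; The construction script runs the parent script, then sets the Cube and Sphere material from AssignTeamOnSpawn, using blue for Team1 and red for Team2.
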(event Custom|ToggleSelectionRing
  (params (bShow :type Boolean))
  (Rendering|SetVisibility (Variables|Default|GetUnitSelectionRing) bShow false))

(event EventTick
  (params (DeltaSeconds :type Float%20%28single-precision%29)))

(event EventBeginPlay
  (|CallParentFunction)
  (EventDispatchers|BindEventtoToggleSelectionRing (Variables|Default|GetUnitInformationComponent) (delegate Custom|ToggleSelectionRing)))

(fn ConstructionScript
  (|CallParentFunction)
  (Rendering|Material|SetMaterial (Variables|Default|GetCube) 0 (Utilities|Select :Index (Variables|Default|GetAssignTeamOnSpawn) :None 0 :EnvironmentTeam 0 :Team1 "/Game/Assets/Materials/Basic/MI_Basic_Blue.MI_Basic_Blue" :Team2 "/Game/Assets/Materials/Basic/MI_Basic_Red.MI_Basic_Red")))