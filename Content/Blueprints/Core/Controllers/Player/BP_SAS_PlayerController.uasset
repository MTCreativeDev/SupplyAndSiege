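; BP_SAS_PlayerController is the player controller that sets up input and the on-screen UI when play begins.
; On BeginPlay it adds the IMC_PlayerMovement Enhanced Input mapping context, then creates WBP_PlayerScreen, stores it and adds it to the viewport.
; It switches to Game and UI input mode focused on that widget, with the mouse locked to the viewport and the cursor visible.
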(event EventBeginPlay
  (bind _self self)
  (Input|AddMappingContext (PlayerController|LocalPlayerSubsystems|GetEnhancedInputLocalPlayerSubsystem self) "/Game/Blueprints/Core/Input/IMC_PlayerMovement.IMC_PlayerMovement" 0 "(bIgnoreAllPressedKeysUntilRelease=True,bForceImmediately=False,bNotifyUserSettings=False)")
  (bind _returnvalue (UserInterface|CreateWidget "/Game/Blueprints/Widgets/WBP_PlayerScreen.WBP_PlayerScreen_C" self))
  (bind _output_get (Variables|Default|SetPlayerScreen _returnvalue))
  (UserInterface|Viewport|AddtoViewport _output_get 0)
  (Input|SetInputModeGameandUI _self (Variables|Default|GetPlayerScreen) "LockAlways" false false)
  (Variables|Default|SetbShowMouseCursor _self true))

(event EventTick
  (params (DeltaSeconds :type Float%20%28single-precision%29)))

(fn ConstructionScript)