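; Display actor that cycles through a list of static and skeletal meshes, showing each with its name on a text render while continuously spinning.
; UpdateMesh shows the component matching the current item's type and applies its asset, scale, location and label.
; After each delay, the index advances with wraparound and the DisplayMovement timeline slides the display along X.
; A timeline event track swaps the mesh during the slide, and completion restarts the loop.
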(event Custom|UpdateDisplay
  (params (BypassMovement :type Boolean))
  (if BypassMovement
    (CallFunction|UpdateMesh)
    (Utilities|FlowControl|Delay 4.0 :!label _label)
    (CallFunction|IncrementItem)
    (bind _movement (Timeline|DisplayMovement PlayFromStart)
      (:Update
        (Transformation|SetRelativeLocation (Variables|Default|GetLocation) (Math|Vector|MakeVector _movement 0.0 0.0) false false))
      (:Finished
        (goto _label))
      (:UpdateMesh
        (CallFunction|UpdateMesh)))
    (else
      (Timeline|DisplayMovement PlayFromStart))))

(event EventBeginPlay
  (CallFunction|UpdateDisplay true))

(event EventTick
  (params (DeltaSeconds :type Float%20%28single-precision%29))
  (bind _rotator (Variables|Default|GetRotator))
  (bind _relativerotation (Variables|/Script/Engine.SceneComponent|GetRelativeRotation _rotator))
  (Transformation|SetRelativeRotation (Variables|Default|GetRotator) (Math|Rotator|MakeRotator (.roll _relativerotation) (.pitch _relativerotation) (+ (.yaw _relativerotation) 1.5)) false false))

(fn ConstructionScript)

(fn UpdateMesh
  (bind _showcaseitems (Variables|Default|GetShowcaseItems))
  (bind _currentindex (Variables|Default|GetCurrentIndex))
  (bind _output (Utilities|Array|Get(acopy) _showcaseitems _currentindex))
  (LocalVariables|SetNewData _output)
  (switch Utilities|FlowControl|Switch|SwitchonEMeshType (Variables|/Script/SupplyAndSiege.SAS_ShowcaseData|GetMeshType _output)
    (:StaticMesh
      (Development|SetHiddeninGame (Variables|Default|GetStaticMesh) false false)
      (Development|SetHiddeninGame (Variables|Default|GetSkeletalMesh) true false)
      (Components|StaticMesh|SetStaticMesh (Variables|Default|GetStaticMesh) (Variables|/Script/SupplyAndSiege.SAS_ShowcaseData|GetStaticMesh (LocalVariables|GetNewData)))
      (Transformation|SetRelativeScale3D (Variables|Default|GetStaticMesh) (Variables|/Script/SupplyAndSiege.SAS_ShowcaseData|GetScale (LocalVariables|GetNewData)))
      (Transformation|SetRelativeLocation (Variables|Default|GetStaticMesh) (Variables|/Script/SupplyAndSiege.SAS_ShowcaseData|GetLocation (LocalVariables|GetNewData)) false false))
    (:SkeletalMesh
      (Development|SetHiddeninGame (Variables|Default|GetStaticMesh) true false)
      (Development|SetHiddeninGame (Variables|Default|GetSkeletalMesh) false false)
      (Components|SkeletalMesh|SetSkeletalMeshAsset (Variables|Default|GetSkeletalMesh) (Variables|/Script/SupplyAndSiege.SAS_ShowcaseData|GetSkeletalMesh (LocalVariables|GetNewData)))
      (Transformation|SetRelativeScale3D (Variables|Default|GetSkeletalMesh) (Variables|/Script/SupplyAndSiege.SAS_ShowcaseData|GetScale (LocalVariables|GetNewData)))
      (Transformation|SetRelativeLocation (Variables|Default|GetSkeletalMesh) (Variables|/Script/SupplyAndSiege.SAS_ShowcaseData|GetLocation (LocalVariables|GetNewData)) false false)))
  (Rendering|Components|TextRender|SetText (Variables|Default|GetTextRender) (Utilities|Text|ToText(Name) (Variables|/Script/SupplyAndSiege.SAS_ShowcaseData|GetDisplayName (LocalVariables|GetNewData)))))

(fn IncrementItem
  (bind _result (Math|Integer|IncrementInt (Variables|Default|GetCurrentIndex))
    (:%20%20
      (if (> _result (Utilities|Array|LastIndex (Variables|Default|GetShowcaseItems)))
        (Variables|Default|SetCurrentIndex 0)))))