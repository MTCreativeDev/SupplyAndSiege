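; BP_Test_ResourcePCG is a test actor that reports itself as a Resource click target.
; On BeginPlay it rebuilds TempInstanceLocations from its Hierarchical Instanced Static Mesh components, adding one local-space location per instance.
; The transform lookup always uses instance index 0, so each component's first location repeats for its whole instance count.
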(event EventBeginPlay
  (Utilities|Array|Clear (Variables|Default|GetTemp_InstanceLocations))
  (for _array_element (Actor|GetComponentsByClass "/Script/Engine.HierarchicalInstancedStaticMeshComponent")
    (for _index (range 0 (- (Components|InstancedStaticMesh|GetInstanceCount _array_element) 1))
      (Utilities|Array|Add (Variables|Default|GetTemp_InstanceLocations) (.Location (Math|Transform|BreakTransform (.OutInstanceTransform (Components|InstancedStaticMesh|GetInstanceTransform _array_element 0 false))))))))

(event Collision|EventActorBeginOverlap
  (params (OtherActor :type Actor%20Object%20Reference)))

(event EventTick
  (params (DeltaSeconds :type Float%20%28single-precision%29)))

(fn ConstructionScript)

(fn GetClickTargetType
  (return "Resource"))